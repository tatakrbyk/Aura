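; Base enemy character Blueprint that handles spawn scale-in, facing targets, dissolve effects and loot drops.
; Timelines grow the mesh on BeginPlay and drive the Dissolve parameter on body and weapon materials, while Motion Warping receives the FacingTarget location.
; SpawnLoot gets items from loot tiers, then a looping timer spawns them one by one in an evenly spaced ring at random distances.
; Spawned AuraEffectActors take the enemy's Level; the LootLevelOverride branch does nothing.
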(event Custom|SpawnLootItem
  (bind _lootitems (Variables|Default|GetLootItems))
  (bind _spawnlootcount (Variables|Default|GetSpawnLootCount))
  (bind _output (Utilities|Array|Get(acopy) _lootitems _spawnlootcount))
  (bind (_lootclass _blootleveloverride) (Utilities|Struct|BreakLootItem _output))
  (if (< (Variables|Default|GetSpawnLootCount) (Utilities|Array|Length (Variables|Default|GetLootItems)))
    (bind _returnvalue (Game|SpawnActorfromClass _lootclass (CallFunction|GetLootTransform (Variables|Default|GetSpawnLootCount)) "AlwaysSpawn" "MultiplyWithRoot" 0 0))
    (bind _asaura_effect_actor (Utilities|Casting|CastToAuraEffectActor _returnvalue)
      (:then
        (Variables|/Script/Aura.AuraEffectActor|SetActorLevel _asaura_effect_actor (Math|Conversions|ToFloat(Integer) (Variables|Default|GetLevel)))
        (if _blootleveloverride
          _
          (else
            _)))
      (:CastFailed
        _))
    (Math|Integer|IncrementInt (Variables|Default|GetSpawnLootCount))
    (else
      (Utilities|Time|ClearandInvalidateTimerbyHandle (Variables|Default|GetLootTimerHandle)))))

(event EventBeginPlay
  (bind _scaletrack (Timeline|SpawnTimeline Play)
    (:Update
      (Transformation|SetRelativeScale3D (Variables|Character|GetMesh) (Math|Vector|MakeVector _scaletrack _scaletrack _scaletrack)))))

(event EventSpawnLoot
  (bind _returnvalue (Class|AuraAbilitySystemLibrary|GetLootTiers))
  (Utilities|IsValid _returnvalue
    (:Is%20Valid
      (bind _returnvalue_2 (Class|LootTiers|GetLootItems _returnvalue))
      (bind _output_get (Variables|Default|SetLootItems _returnvalue_2))
      (Variables|Default|SetLootRotations (CallFunction|GetLootRotations _output_get))
      (Variables|Default|SetSpawnLootCount 0)
      (bind _returnvalue_3 (Utilities|Time|SetTimerbyEvent (delegate Custom|SpawnLootItem) 0.1 true))
      (Variables|Default|SetLootTimerHandle _returnvalue_3)
      (CallFunction|SpawnLootItem))))

(event EventStartDissolveTimeLine
  (params (DynamicMaterialInstance :type Material%20Instance%20Dynamic%20Object%20Reference))
  ;[1 1 1] AuraCharacterBase
  (bind _dissolvetrack (Timeline|DissolveTimeLine Play)
    (:Update
      (Rendering|Material|SetScalarParameterValue DynamicMaterialInstance "Dissolve" _dissolvetrack :!class /Script/Engine.MaterialInstanceDynamic))))

(event EventStartWeaponDissolveTimeline
  (params (DynamicMaterialInstance :type Material%20Instance%20Dynamic%20Object%20Reference))
  ;[1 1 1] AuraCharacterBase
  (bind _weapondissolvetrack (Timeline|WeaponDissolveTimeLine Play)
    (:Update
      (Rendering|Material|SetScalarParameterValue DynamicMaterialInstance "Dissolve" _weapondissolvetrack :!class /Script/Engine.MaterialInstanceDynamic))))

(event EventUpdateFacingTarget
  (params (Target :type Vector%20%28by%20ref%29 :default "0, 0, 0"))
  (Class|MotionWarpingComponent|AddorUpdateWarpTargetfromLocation (Variables|Default|GetMotionWarping) "FacingTarget" Target))

(fn ConstructionScript)

(fn GetLootRotations
  (params (TargetArray :type Array%20of%20Loot%20Item%20Structures))
  (return (Class|AuraAbilitySystemLibrary|EvenlySpacedRotators (Transformation|GetActorForwardVector) (Math|Vector|VectorUp) 3.6e+02 (Utilities|Array|Length TargetArray))))

(fn GetLootTransform
  (params (LoopCount :type Integer))
  (bind _lootrotations (Variables|Default|GetLootRotations))
  (bind _output (Utilities|Array|Get(acopy) _lootrotations LoopCount))
  (return (Math|Transform|MakeTransform (+ (* (Math|Vector|GetForwardVector _output) (Math|Random|RandomFloatinRange (LocalVariables|GetMinSpawnDistance) (LocalVariables|GetMaxSpawnDistance))) (Transformation|GetActorLocation)) _output)))